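; BP_WeaponManager is a player character component that manages the single weapon the character holds in a networked game.
; CreateWeapon spawns and AddWeapon adopts a weapon, both routing through CheckCurrentWeapon, which drops any held weapon before assigning ownership.
; Dropping clears ownership and moves the weapon in front of the character.
; The character reference is cached on the server, and CurrentWeapon's RepNotify calls CallWeaponSelected when it changes.
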(event `CharacterSet`
  (if (`KismetSystemLibrary.IsServer`)
    (bind _asbp_player_character (cast `/Game/BluePrints/Player/BP_PlayerCharacter` (`self.GetOwner`))
      (:`then`
        (set `self.Characher` _asbp_player_character))
      (:`CastFailed`
        (`KismetSystemLibrary.PrintString` "Not Cast BP_PlayerCaharacter")))))

(event `ManagerDropWeapon`
  ;[1 1 1] ManagerDropWeapon
  (`self.CurrentWeapon`
    (:`then`
      (`self.ServerDropWeapon`))
    (:`else`)))

(event `ServerDropWeapon`
  ;[1 1 1] ManagerDropWeapon
  (bind _currentweapon (`self.CurrentWeapon`)
    (:`then`
      (`self.DropWeapon` _currentweapon))
    (:`else`)))

(fn `AddWeapon`
  (params (Weapon :type "/Game/BluePrints/Weapons/BP_Weapon Object Reference"))
  (locals (L_Weapon :type "/Game/BluePrints/Weapons/BP_Weapon Object Reference"))
  (bind _characher (`self.Characher`))
  (bind _output_get (set `local.L_Weapon` Weapon))
  (set `Actor.Instigator` _characher _output_get)
  (`Actor.SetOwner` (`local.L_Weapon`) (`Pawn.GetController` _characher))
  (`self.Check Current Weapon` (`/Game/BluePrints/Player/BP_PlayerCharacter.BP_WeaponManager` _characher) (`local.L_Weapon`))
  (add `/Game/BluePrints/Player/BP_PlayerCharacter.CharDead` (`self.Characher`) (`|CreateDelegate` :!event `DeleteWeapon`)))

(fn `Check Current Weapon`
  (params (Weapon :type "/Game/BluePrints/Weapons/BP_Weapon Object Reference"))
  (locals (L_Weapon :type "/Game/BluePrints/Weapons/BP_Weapon Object Reference"))
  (set `local.L_Weapon` Weapon)
  (`self.CurrentWeapon`
    (:`then`
      (`self.DropWeapon` (`self.CurrentWeapon`))
      (set `/Game/BluePrints/Weapons/BP_Weapon.WeaponOwner` (`self.Characher`) (`local.L_Weapon`))
      (set `self.CurrentWeapon` (`local.L_Weapon`)))
    (:`else`
      (set `/Game/BluePrints/Weapons/BP_Weapon.WeaponOwner` (`self.Characher`) (`local.L_Weapon`))
      (set `self.CurrentWeapon` (`local.L_Weapon`)))))

(fn `Create Weapon`
  (params (Class :type "/Game/BluePrints/Weapons/BP_Weapon Class Reference"))
  (bind _characher (`self.Characher`))
  (bind _returnvalue (`|SpawnActorFromClass` Class (`KismetMathLibrary.MakeTransform` (0.0 0.0 0.0)) "AlwaysSpawn" "OverrideRootScale" (`Pawn.GetController` _characher) _characher _characher))
  (`self.Check Current Weapon` (`/Game/BluePrints/Player/BP_PlayerCharacter.BP_WeaponManager` (`self.Characher`)) _returnvalue))

(fn `DeleteWeapon`
  (bind _currentweapon (`self.CurrentWeapon`)
    (:`then`
      (`Actor.K2_DestroyActor` _currentweapon))
    (:`else`)))

(fn `DropWeapon`
  (params (Weapon :type "/Game/BluePrints/Weapons/BP_Weapon Object Reference"))
  (locals (L_Weapon :type "/Game/BluePrints/Weapons/BP_Weapon Object Reference"))
  (bind _characher (`self.Characher`))
  (bind _output_get (set `local.L_Weapon` Weapon))
  (if (== (`/Game/BluePrints/Weapons/BP_Weapon.WeaponOwner` _output_get) (`self.Characher`))
    (set `/Game/BluePrints/Weapons/BP_Weapon.WeaponOwner` null (`local.L_Weapon`))
    (set `self.CurrentWeapon` null)
    (`Actor.K2_SetActorLocation` (`local.L_Weapon`) (+ (`SceneComponent.K2_GetComponentLocation` (`Actor.RootComponent` _characher)) (* (`SceneComponent.GetForwardVector` (`Actor.RootComponent` _characher)) 100.0)) false false)))

(fn `IsEqualWeaponClass`
  (params (Weapon :type "/Game/BluePrints/Weapons/BP_Weapon Object Reference"))
  (returns (out :type Boolean))
  (return (== (`GameplayStatics.GetObjectClass` Weapon) (`GameplayStatics.GetObjectClass` (`self.CurrentWeapon`)))))

(fn `OnRep_CurrentWeapon`
  (`self.WeaponSelected` (`self.CurrentWeapon`)))