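; BP_HealthManager is a player component that tracks health and handles damage and death.
; On the server it binds to the owning BP_PlayerCharacter's point damage event, asking the game mode whether each hit counts, which filters friendly fire.
; Accepted damage passes through a math expression before reducing Health.
; At zero health it flags the character Dead and reports killer, victim and damage causer to BP_BaseGameMode.
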(event Custom|OnPlayerTakePointDamage
  (params (DamagedActor :type Actor%20Object%20Reference) (Damage :type Float%20%28single-precision%29) (InstigatedBy :type Controller%20Object%20Reference) (HitLocation :type Vector) (FHitComponent :type Primitive%20Component%20Object%20Reference) (BoneName :type Name) (ShotFromDirection :type Vector) (DamageType :type Damage%20Type%20Object%20Reference) (DamageCauser :type Actor%20Object%20Reference))
  (bind _asbp_base_player_controller (Utilities|Casting|CastToBP_BasePlayerController InstigatedBy))
  (if (not (Variables|/Game/BluePrints/Player/BP_PlayerCharacter.BP_PlayerCharacter_C|GetDead (Variables|Default|GetCharacher)))
    (if (Default|ShouldDamagePlayer (CallFunction|GetBaseGameMode) (CallFunction|GetBasePlayerController (Variables|Default|GetCharacher)) _asbp_base_player_controller)
      (CallFunction|ApplyDamage Damage)
      (if (and (not (Variables|/Game/BluePrints/Player/BP_PlayerCharacter.BP_PlayerCharacter_C|GetDead (Variables|Default|GetCharacher))) (<= (Variables|Default|GetHealth) 0.0))
        (Variables|/Game/BluePrints/Player/BP_PlayerCharacter.BP_PlayerCharacter_C|SetDead (Variables|Default|GetCharacher) true)
        (bind _asbp_base_game_mode (Utilities|Casting|CastToBP_BaseGameMode (Game|GetGameMode)))
        (Default|CharacterDead _asbp_base_game_mode _asbp_base_player_controller (Variables|Default|GetCharacher) DamageCauser))
      (else
        (Development|PrintString "Урон по своим")))
    (else
      (Development|PrintString "Урон приходит на мертвого"))))

(event EventTick
  (params (DeltaSeconds :type Float%20%28single-precision%29)))

(event EventBeginPlay
  (Variables|Default|SetHealth (Variables|Default|GetMaxHealth))
  (if (Networking|IsServer)
    (bind _asbp_player_character (Utilities|Casting|CastToBP_PlayerCharacter (Components|GetOwner))
      (:then
        (bind _output_get (Variables|Default|SetCharacher _asbp_player_character))
        (EventDispatchers|AssignOnTakePointDamage _output_get (EventDispatchers|CreateEvent :!event Custom|OnPlayerTakePointDamage)))
      (:CastFailed
        (Development|PrintString "Not Cast BP_PlayerCaharacter")))))

(fn ApplyDamage
  (params (Damage :type Float%20%28single-precision%29))
  (bind _output_get (LocalVariables|SetL_damage (|(Damage*(1-({561F3ACF-41DE-A2F7-00A4-DF974B8C79B4}/100))) Damage)))
  (Development|PrintString (Utilities|String|Append "Damage: " (Utilities|String|ToString(Float) _output_get)) true true "(R=0.000000,G=0.144330,B=1.000000,A=1.000000)")
  (Variables|Default|SetHealth (- (Variables|Default|GetHealth) (LocalVariables|GetL_damage))))

(fn GetHealth
  (return (Variables|Default|GetHealth)))