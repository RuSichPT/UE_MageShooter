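; Game component that runs a timed, replicated map vote among players.
; StartVote loads map names from DT_Maps and enables a once-per-second tick that counts down TimeOfVote, then stops the vote.
; SetVote stores each player's choice at their PlayerArray index.
; RepNotifies on Maps and VoteInProgress broadcast the map list, vote start, and vote end with the most-voted map.
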(event `self.ReceiveTick`
  (params (DeltaSeconds :type "Float (single-precision)"))
  (bind _result (`/Engine/EditorBlueprintResources/StandardMacros.DecrementInt` (`self.TimeOfVote`))
    (:`  `
      (if (<= _result 0)
        (`self.StopVote`)))))

(fn `Get Map Votes`
  (params (MapIndex :type Integer))
  (returns (Votes :type Integer))
  (locals (L_Votes :type Integer))
  (for _array_element (`self.PlayersVotes`)
    (if (== MapIndex _array_element)
      (`/Engine/EditorBlueprintResources/StandardMacros.IncrementInt` (`local.L_Votes`))))
  (return (`local.L_Votes`)))

(fn `GetVotedMap`
  (returns (MapName :type "Name (by ref)"))
  (locals (L_MaxVotesIndex :type Integer) (L_MaxVotes :type Integer))
  (if (!= (`KismetArrayLibrary.Array_Length` (`self.Maps`)) 0)
    (for (_ _array_index) (`self.Maps`)
      (bind _votes (`self.Get Map Votes` _array_index))
      (if (> _votes (`local.L_MaxVotes`))
        (set `local.L_MaxVotes` _votes)
        (set `local.L_MaxVotesIndex` _array_index)))
    (return (`|GetArrayItem` (`self.Maps`) (`local.L_MaxVotesIndex`)))
    (else
      (return "None"))))

(fn `Init Maps`
  (bind _outrownames (`DataTableFunctionLibrary.GetDataTableRowNames` "/Game/Data/DT_Maps.DT_Maps"))
  (set `self.Maps` _outrownames))

(fn `OnRep_Maps`
  (`self.MapGenerated` (`self.Maps`)))

(fn `OnRep_VoteInProgress`
  (if (`self.VoteInProgress`)
    (`self.VoteStarted`)
    (else
      (`self.VoteEnded` (`self.GetVotedMap`)))))

(fn `SetVote`
  (params (MapIndex :type Integer) (PlayerState :type "/Game/BluePrints/Player/BP_Player_State Object Reference"))
  (`KismetArrayLibrary.Array_Set` (`self.PlayersVotes`) (`KismetArrayLibrary.Array_Find` (`GameStateBase.PlayerArray` (`/Game/BluePrints/Libs/Functions/BP_GlobalGetters.GetBaseGameState`)) PlayerState) MapIndex true))

(fn `StartVote`
  (`self.SetComponentTickEnabled` true)
  (`self.Init Maps`)
  (set `self.VoteInProgress` true))

(fn `StopVote`
  (`self.SetComponentTickEnabled` false)
  (set `self.VoteInProgress` false))