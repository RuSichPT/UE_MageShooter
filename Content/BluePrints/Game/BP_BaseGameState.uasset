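; Base game state that tracks match phase and timing, moving from pre-start countdown through the game to end.
; A once-per-second, authority-only Tick counts down to MatchStart, then advances match time and reports the limit to the base game mode.
; The game mode's match-ended event sets the end phase; multicasts relay start and end to match dispatchers.
; StartGameTimer offers a looping timer for match time but is not called here.
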(event `self.ReceiveBeginPlay`
  (`/Engine/EditorBlueprintResources/ActorMacros.Switch Has Authority`
    (:`Authority`
      (add `/Game/BluePrints/Game/BP_BaseGameMode.MatchEndedServer` (`/Game/BluePrints/Libs/Functions/BP_GlobalGetters.GetBaseGameMode`) (delegate `OnEndedMatch`)))))

(event `OnEndedMatch`
  (params (Reason :type String))
  (`self.MulticastEndedMatch` Reason)
  (set `self.GameState` "NewEnumerator2"))

(event `MulticastStartedMatch`
  (`self.MatchStarted`))

(event `MulticastEndedMatch`
  (params (Reason :type String))
  (`self.MatchEnded` Reason))

(event `self.ReceiveTick`
  (params (DeltaSeconds :type "Float (single-precision)"))
  (`/Engine/EditorBlueprintResources/ActorMacros.Switch Has Authority`
    (:`Authority`
      (switch `/Game/Data/E_GameState` (`self.GameState`)
        (:`NewEnumerator0`
          (bind _result (`/Engine/EditorBlueprintResources/StandardMacros.DecrementInt` (`self.TimeBeforeStart`))
            (:`  `
              (if (<= _result 0)
                (`/Game/BluePrints/Game/BP_BaseGameMode.Match Start` (`/Game/BluePrints/Libs/Functions/BP_GlobalGetters.GetBaseGameMode`))
                (set `self.GameState` "NewEnumerator1")
                (`self.MulticastStartedMatch`)))))
        (:`NewEnumerator1`
          (`self.Match Time Tick`))))))

(fn `Match Time Tick`
  (set `self.MatchTme` (+ (`self.MatchTme`) (`KismetMathLibrary.MakeTimespan` 0 0 0 1)))
  (if (>= (`self.MatchTme`) (`/Game/BluePrints/Game/BP_BaseGameMode.LimitTime` (`/Game/BluePrints/Libs/Functions/BP_GlobalGetters.GetBaseGameMode`)))
    (`/Game/BluePrints/Game/BP_BaseGameMode.MatchTimeEnd` (`/Game/BluePrints/Libs/Functions/BP_GlobalGetters.GetBaseGameMode`))))

(fn `Start Game Timer`
  (bind _returnvalue (`KismetSystemLibrary.K2_SetTimer` null "Match Time Tick" 1.0 true))
  (set `self.MatchTimer` _returnvalue))

(fn `UserConstructionScript`)