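; Team-based game mode that overrides spawn selection, damage rules, scoring and the match end condition of its parent.
; Spawns are limited to free BP_Player_Start actors of the player's team, and teammate damage requires friendly fire to be enabled.
; Statistic updates add a point to the instigator's team for enemies and subtract one for teammates through the team game state.
; Character deaths stop the match once the instigator's team reaches the optional point limit.
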(fn `CharacterDead`
  (params (`Death Instigator` :type "/Game/BluePrints/Player/BP_BasePlayerController Object Reference") (`Dead Character` :type "/Game/BluePrints/Player/BP_PlayerCharacter Object Reference") (`Death Caused By` :type "Actor Object Reference"))
  (`parent.CharacterDead` `Death Instigator` `Dead Character` `Death Caused By`)
  (if (`self.LimitByTeamPoints`)
    (if (>= (`/Game/BluePrints/Game/BP_TeamGameState.GetTeamPoints` (`/Game/BluePrints/Libs/Functions/BP_GlobalGetters.GetTeamGameState`) (`/Game/BluePrints/Player/BP_TeamPlayer_State.Team` (`/Game/BluePrints/Libs/Functions/BP_GlobalGetters.GetTeamPlayerStateByController` `Death Instigator`))) (`self.LimitTeamPoints`))
      (`self.Match Stop` "LimitTeamPoints"))))

(fn `getFreeStartPlayer`
  (params (Player :type "/Game/BluePrints/Player/BP_BasePlayerController Object Reference"))
  (returns (FreeStartPlayer :type "Array of /Game/BluePrints/Game/BP_Player_Start Object Reference"))
  (locals (L_FreeStartPlayer :type "Array of /Game/BluePrints/Game/BP_Player_Start Object Reference"))
  (bind _outactors (`GameplayStatics.GetAllActorsOfClass` "/Game/BluePrints/Game/BP_Player_Start.BP_Player_Start_C"))
  (for _array_element _outactors
    (if (and (`|EnumEquality` (`/Game/BluePrints/Player/BP_TeamPlayer_State.Team` (`/Game/BluePrints/Libs/Functions/BP_GlobalGetters.GetTeamPlayerStateByController` Player)) (`/Game/BluePrints/Game/BP_Player_Start.Team` _array_element)) (`/Game/BluePrints/Game/BP_Player_Start.Is Free` _array_element))
      (`KismetArrayLibrary.Array_Add` (`local.L_FreeStartPlayer`) _array_element)))
  (return (`local.L_FreeStartPlayer`)))

(fn `IsEnemy`
  (params (FirstPlayer :type "/Game/BluePrints/Player/BP_BasePlayerController Object Reference") (SecondPlayer :type "/Game/BluePrints/Player/BP_BasePlayerController Object Reference"))
  (returns (Out :type Boolean))
  (return (`|EnumInequality` (`/Game/BluePrints/Player/BP_TeamPlayer_State.Team` (`/Game/BluePrints/Libs/Functions/BP_GlobalGetters.GetTeamPlayerStateByController` FirstPlayer)) (`/Game/BluePrints/Player/BP_TeamPlayer_State.Team` (`/Game/BluePrints/Libs/Functions/BP_GlobalGetters.GetTeamPlayerStateByController` SecondPlayer)))))

(fn `ShouldDamagePlayer`
  (params (Player :type "/Game/BluePrints/Player/BP_BasePlayerController Object Reference") (Instigator :type "/Game/BluePrints/Player/BP_BasePlayerController Object Reference"))
  (returns (Out :type Boolean))
  (if (`self.AllowFrendlyFire`)
    (return true)
    (else
      (return (`|EnumInequality` (`/Game/BluePrints/Player/BP_TeamPlayer_State.Team` (`/Game/BluePrints/Libs/Functions/BP_GlobalGetters.GetTeamPlayerStateByController` Player)) (`/Game/BluePrints/Player/BP_TeamPlayer_State.Team` (`/Game/BluePrints/Libs/Functions/BP_GlobalGetters.GetTeamPlayerStateByController` Instigator)))))))

(fn `UpdateStatisticPoints`
  (params (Player :type "/Game/BluePrints/Player/BP_BasePlayerController Object Reference") (Instigator :type "/Game/BluePrints/Player/BP_BasePlayerController Object Reference"))
  (`parent.UpdateStatisticPoints` Player Instigator)
  (`/Engine/EditorBlueprintResources/StandardMacros.IsValid` Instigator
    (:`Is Valid`
      (if (`self.IsEnemy` Player Instigator)
        (`/Game/BluePrints/Game/BP_TeamGameState.Set Team Points` (`/Game/BluePrints/Libs/Functions/BP_GlobalGetters.GetTeamGameState`) (`/Game/BluePrints/Player/BP_TeamPlayer_State.Team` (`/Game/BluePrints/Libs/Functions/BP_GlobalGetters.GetTeamPlayerStateByController` Instigator)) 1)
        (else
          (`/Game/BluePrints/Game/BP_TeamGameState.Set Team Points` (`/Game/BluePrints/Libs/Functions/BP_GlobalGetters.GetTeamGameState`) (`/Game/BluePrints/Player/BP_TeamPlayer_State.Team` (`/Game/BluePrints/Libs/Functions/BP_GlobalGetters.GetTeamPlayerStateByController` Instigator)) -1))))))

(fn `UserConstructionScript`
  (`parent.UserConstructionScript`))