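; BP_Player_Start is a spawn point that creates a player character and tracks whether one is occupying it.
; SpawnCharacter destroys the given controller's current pawn, spawns a new BP_PlayerCharacter at the start's transform, possesses it and records it as CharacterInside.
; Capsule overlap events set and clear CharacterInside, and IsFree reports the point free when that reference is invalid.
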(event `self.CapsuleComponent.OnComponentBeginOverlap`
  (params (OverlappedComponent :type "PrimitiveComponent Object Reference") (OtherActor :type "Actor Object Reference") (OtherComp :type "PrimitiveComponent Object Reference") (OtherBodyIndex :type Integer) (bFromSweep :type Boolean) (SweepResult :type "HitResult Structure (by ref)"))
  (bind _asbp_player_character (cast `/Game/BluePrints/Player/BP_PlayerCharacter` OtherActor))
  (set `self.Character Inside` _asbp_player_character))

(event `self.CapsuleComponent.OnComponentEndOverlap`
  (params (OverlappedComponent :type "PrimitiveComponent Object Reference") (OtherActor :type "Actor Object Reference") (OtherComp :type "PrimitiveComponent Object Reference") (OtherBodyIndex :type Integer))
  (if (== OtherActor (`self.Character Inside`))
    (set `self.Character Inside` null)))

(fn `Is Free`
  (returns (Free :type Boolean))
  (`self.Character Inside`
    (:`then`
      (return false))
    (:`else`
      (return true))))

(fn `Spawn Character`
  (params (Player :type "/Game/BluePrints/Player/BP_BasePlayerController Object Reference"))
  (returns (Character :type "/Game/BluePrints/Player/BP_PlayerCharacter Object Reference"))
  (bind _returnvalue (`Controller.K2_GetPawn` Player))
  (if (`KismetSystemLibrary.IsValid` Player)
    (`|ExecutionSequence`
      (:`then_0`
        (if (`KismetSystemLibrary.IsValid` _returnvalue)
          (`self.K2_DestroyActor` _returnvalue)))
      (:`then_1`
        (bind _returnvalue_2 (`|SpawnActorFromClass` "/Game/BluePrints/Player/BP_PlayerCharacter.BP_PlayerCharacter_C" (`self.GetTransform`) "Undefined" "OverrideRootScale" Player null))
        (bind _output_get (set `self.Character Inside` _returnvalue_2))
        (`Controller.Possess` Player _output_get)
        (return _output_get)))
    (else
      (`KismetSystemLibrary.PrintString` "Not Player Controller"))))

(fn `UserConstructionScript`)