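; Game State for a two-team mode that tracks each team's score and reports which players belong to a team.
; SetTeamPoints adds the given value to the team's entry in the TeamPoints map, then mirrors the total into TeamPointsArray, which is sized at BeginPlay.
; GetTeamPoints reads that array through a team-to-index select.
; GetPlayersOfTeam filters PlayerArray by each BP_TeamPlayer_State's Team.
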(event `self.ReceiveBeginPlay`
  (`parent.ReceiveBeginPlay`)
  (`KismetArrayLibrary.Array_Resize` (`self.TeamPointsArray`) (`BlueprintMapLibrary.Map_Length` (`self.TeamPoints`))))

(fn `GetPlayersOfTeam`
  (params (Team :type "/Game/Data/E_Team Enum" :default "NewEnumerator0"))
  (returns (PlayersOfTeam :type "Array of /Game/BluePrints/Player/BP_TeamPlayer_State Object Reference"))
  (locals (L_PlayersOfTeam :type "Array of /Game/BluePrints/Player/BP_TeamPlayer_State Object Reference"))
  (for _array_element (`self.PlayerArray`)
    (bind _asbp_team_player_state (cast `/Game/BluePrints/Player/BP_TeamPlayer_State` _array_element :!pure true))
    (if (`|EnumEquality` (`/Game/BluePrints/Player/BP_TeamPlayer_State.Team` _asbp_team_player_state) Team)
      (`KismetArrayLibrary.Array_Add` (`local.L_PlayersOfTeam`) _asbp_team_player_state)))
  (return (`local.L_PlayersOfTeam`)))

(fn `GetTeamPoints`
  (params (Team :type "/Game/Data/E_Team Enum" :default "NewEnumerator0"))
  (returns (TeamPoints :type Integer))
  (return (`|GetArrayItem` (`self.TeamPointsArray`) (select `/Game/Data/E_Team` Team :`NewEnumerator1` 1))))

(fn `Set Team Points`
  (params (Team :type "/Game/Data/E_Team Enum" :default "NewEnumerator0") (Value :type Integer))
  (`BlueprintMapLibrary.Map_Add` (`self.TeamPoints`) Team (+ (`BlueprintMapLibrary.Map_Find` (`self.TeamPoints`) Team) Value))
  (`KismetArrayLibrary.Array_Set` (`self.TeamPointsArray`) (select `/Game/Data/E_Team` Team :`NewEnumerator1` 1) (`BlueprintMapLibrary.Map_Find` (`self.TeamPoints`) Team)))

(fn `UserConstructionScript`
  (`parent.UserConstructionScript`))