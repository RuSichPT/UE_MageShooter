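; Spectator actor that follows a target character, moving only where it lacks network authority, so it stays still on the server.
; Each tick it interpolates its location toward FollowCharacter with VInterpTo, without sweeping, while that reference is valid.
; One second after BeginPlay it sets the interpolation speed to a fixed value so the follow stops looking smoothed once the initial approach is done.
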(event `self.ReceiveBeginPlay`
  (`parent.ReceiveBeginPlay`)
  (`/Engine/EditorBlueprintResources/ActorMacros.Switch Has Authority` ; На сервере не двигается спектатор
    (:`Remote`
      (`KismetSystemLibrary.Delay` 1.0)
      (set `self.Interp Speed` 20.0) ; Чтобы не было  плавности после приближения
    )))

(event `self.ReceiveTick`
  (params (DeltaSeconds :type "Float (single-precision)"))
  (`parent.ReceiveTick` DeltaSeconds)
  (`/Engine/EditorBlueprintResources/ActorMacros.Switch Has Authority` ; На сервере не двигается спектатор
    (:`Remote`
      (bind _followcharacter (`self.FollowCharacter`)
        (:`then`
          (`self.K2_SetActorLocation` (`KismetMathLibrary.VInterpTo` (`self.K2_GetActorLocation`) (`self.K2_GetActorLocation` _followcharacter) (`GameplayStatics.GetWorldDeltaSeconds`) (`self.Interp Speed`))))
        (:`else`)))))

(fn `UserConstructionScript`
  (`parent.UserConstructionScript`))