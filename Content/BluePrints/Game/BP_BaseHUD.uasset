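; Base HUD that manages the player's screen widgets across match phases: pre-start, in-game HUD, spectate, tab menu, chat and game end.
; BeginPlay creates the pre-start and end screens and binds to game state match events; match start creates the in-game widgets.
; Player state alive and dead events swap HUD and spectate, passing death info to the spectate widget.
; Toggle functions add or remove widgets only when not on the server.
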(event `self.ReceiveDrawHUD`
  (params (SizeX :type Integer) (SizeY :type Integer)))

(event `self.ReceiveBeginPlay`
  (bind _asbp_base_game_state (`/Game/BluePrints/Libs/Functions/BP_GlobalGetters.GetBaseGameState`))
  (`self.CreateAllWidgetPreStartGame`)
  (`self.CreateAllWidgetGameEnd`)
  (`self.TogglePreStartGame` true)
  (add `/Game/BluePrints/Game/BP_BaseGameState.MatchStarted` _asbp_base_game_state (delegate `MatchStarted`))
  (add `/Game/BluePrints/Game/BP_BaseGameState.MatchEnded` _asbp_base_game_state (delegate `MatchEnded`)))

(event `MatchEnded`
  (params (Reason :type String))
  (`self.ToggleHUD` false)
  (`self.ToggleSpectate` false)
  (`self.ToggleTabMenu` false)
  (`self.ToggleGameEnd` true))

(event `MatchStarted`
  (bind _asbp_player_state (`/Game/BluePrints/Libs/Functions/BP_GlobalGetters.GetPlayerStateByController` (`self.GetOwningPlayerController`)))
  (`self.TogglePreStartGame` false)
  (`self.CreateAllWidgetGame`) ; Отображение виджетов\nтолько на  клиенте
  (`self.ToggleHUD` true)
  (`|ExecutionSequence`
    (:`then_0`
      (add `/Game/BluePrints/Player/BP_Player_State.PlayerAlive` _asbp_player_state (delegate `PlayerAlive`)))
    (:`then_1`
      (add `/Game/BluePrints/Player/BP_Player_State.PlayerDead` _asbp_player_state (delegate `PlayerDead`)))))

(event `PlayerAlive`
  (`self.ToggleHUD` true)
  (`self.ToggleSpectate` false))

(event `PlayerDead`
  (params (`Instogator Character` :type "/Game/BluePrints/Player/BP_PlayerCharacter Object Reference") (`Death Caused By` :type "Actor Object Reference") (DeadPlayer :type "/Game/BluePrints/Player/BP_Player_State Object Reference"))
  (`self.ToggleHUD` false)
  (`self.ToggleSpectate` true)
  (if (`|EnumEquality` (`/Game/BluePrints/Game/BP_BaseGameState.GameState` (`/Game/BluePrints/Libs/Functions/BP_GlobalGetters.GetBaseGameState`)) "NewEnumerator1")
    (`/Game/UI/Spectate/W_Spectate.SetInfoDeath` (`self.W_Spectate`) `Instogator Character` `Death Caused By`)))

(fn `CreateAllWidgetGame`
  (bind _returnvalue (`self.GetOwningPlayerController`))
  (bind _returnvalue_2 (`|CreateWidget` (`self.W_Tab_Menu_class`) _returnvalue))
  (set `self.W_Tab_Menu` _returnvalue_2)
  (bind _returnvalue_3 (`|CreateWidget` (`self.W_HUD_class`) _returnvalue))
  (set `self.W_HUD` _returnvalue_3)
  (bind _returnvalue_4 (`|CreateWidget` (`self.W_Spectate_class`) _returnvalue))
  (set `self.W_Spectate` _returnvalue_4)
  (bind _returnvalue_5 (`|CreateWidget` (`self.W_Chat_class`) _returnvalue))
  (bind _output_get (set `self.W_Chat` _returnvalue_5))
  (`UserWidget.AddToViewport` _output_get 0))

(fn `CreateAllWidgetGameEnd`
  (bind _returnvalue (`|CreateWidget` (`self.W_GameEnd_class`) (`self.GetOwningPlayerController`)))
  (set `self.W_GameEnd` _returnvalue))

(fn `CreateAllWidgetPreStartGame`
  (bind _returnvalue (`|CreateWidget` (`self.W_PreStartGame_class`) (`self.GetOwningPlayerController`)))
  (set `self.W_PreStartGame` _returnvalue))

(fn `IsActiveChat`
  (returns (Activate :type Boolean))
  (return (`/Game/UI/General/MessageChat/W_MessageChat.Activate` (`self.W_Chat`))))

(fn `ToggleChat`
  (params (Active :type Boolean))
  (bind _w_chat (`self.W_Chat`))
  (if Active
    (`/Game/UI/General/MessageChat/W_MessageChat.ActivateChat` _w_chat)
    (else
      (`/Game/UI/General/MessageChat/W_MessageChat.DeactivateChat` _w_chat))))

(fn `ToggleGameEnd`
  (params (Show :type Boolean))
  (bind _returnvalue (`KismetSystemLibrary.IsServer`))
  (bind _w_gameend (`self.W_GameEnd`))
  (if Show
    (if (not _returnvalue)
      (`/Engine/EditorBlueprintResources/StandardMacros.IsValid` _w_gameend
        (:`Is Valid`
          (`UserWidget.AddToViewport` _w_gameend 0))))
    (elif (not _returnvalue)
      (`/Engine/EditorBlueprintResources/StandardMacros.IsValid` _w_gameend
        (:`Is Valid`
          (`Widget.RemoveFromParent` _w_gameend))))))

(fn `ToggleHUD`
  (params (Show :type Boolean))
  (bind _returnvalue (`KismetSystemLibrary.IsServer`))
  (bind _w_hud (`self.W_HUD`))
  (if Show
    (if (not _returnvalue)
      (`/Engine/EditorBlueprintResources/StandardMacros.IsValid` _w_hud
        (:`Is Valid`
          (`Widget.RemoveFromParent` _w_hud)
          (`UserWidget.AddToViewport` _w_hud 0))))
    (elif (not _returnvalue)
      (`/Engine/EditorBlueprintResources/StandardMacros.IsValid` _w_hud
        (:`Is Valid`
          (`Widget.RemoveFromParent` _w_hud))))))

(fn `TogglePreStartGame`
  (params (Show :type Boolean))
  (bind _returnvalue (`KismetSystemLibrary.IsServer`))
  (bind _w_prestartgame (`self.W_PreStartGame`))
  (if Show
    (if (not _returnvalue)
      (`/Engine/EditorBlueprintResources/StandardMacros.IsValid` _w_prestartgame
        (:`Is Valid`
          (`UserWidget.AddToViewport` _w_prestartgame 0))))
    (elif (not _returnvalue)
      (`/Engine/EditorBlueprintResources/StandardMacros.IsValid` _w_prestartgame
        (:`Is Valid`
          (`Widget.RemoveFromParent` _w_prestartgame))))))

(fn `ToggleSpectate`
  (params (Show :type Boolean))
  (bind _returnvalue (`KismetSystemLibrary.IsServer`))
  (bind _w_spectate (`self.W_Spectate`))
  (if Show
    (if (`|EnumEquality` (`/Game/BluePrints/Game/BP_BaseGameState.GameState` (`/Game/BluePrints/Libs/Functions/BP_GlobalGetters.GetBaseGameState`)) "NewEnumerator1")
      (if (not _returnvalue)
        (`/Engine/EditorBlueprintResources/StandardMacros.IsValid` _w_spectate
          (:`Is Valid`
            (`UserWidget.AddToViewport` _w_spectate 0)))))
    (elif (not _returnvalue)
      (`/Engine/EditorBlueprintResources/StandardMacros.IsValid` _w_spectate
        (:`Is Valid`
          (`Widget.RemoveFromParent` _w_spectate))))))

(fn `ToggleTabMenu`
  (params (Show :type Boolean))
  (bind _returnvalue (`KismetSystemLibrary.IsServer`))
  (bind _w_tab_menu (`self.W_Tab_Menu`))
  (if Show
    (if (not _returnvalue)
      (`/Engine/EditorBlueprintResources/StandardMacros.IsValid` _w_tab_menu
        (:`Is Valid`
          (`UserWidget.AddToViewport` _w_tab_menu 0))))
    (elif (not _returnvalue)
      (`/Engine/EditorBlueprintResources/StandardMacros.IsValid` _w_tab_menu
        (:`Is Valid`
          (`Widget.RemoveFromParent` _w_tab_menu))))))

(fn `UserConstructionScript`)