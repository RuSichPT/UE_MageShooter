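; BP_DeathMatchGameMode is a deathmatch game mode that can end the match when a player reaches a kill limit.
; It overrides CharacterDead, calls the parent, then, if LimitByKills is on, reads the instigator's BP_Player_State kills.
; Reaching LimitKills calls MatchStop with a "LimitKills" reason, while a death without a valid instigator only prints a debug message in Russian.
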(fn `CharacterDead`
  (params (`Death Instigator` :type "/Game/BluePrints/Player/BP_BasePlayerController Object Reference") (`Dead Character` :type "/Game/BluePrints/Player/BP_PlayerCharacter Object Reference") (`Death Caused By` :type "Actor Object Reference"))
  (`parent.CharacterDead` `Death Instigator` `Dead Character` `Death Caused By`)
  (if (`self.LimitByKills`)
    (`/Engine/EditorBlueprintResources/StandardMacros.IsValid` `Death Instigator`
      (:`Is Valid`
        (bind _playerstate (`Controller.PlayerState` `Death Instigator`)
          (:`then`
            (bind _asbp_player_state (cast `/Game/BluePrints/Player/BP_Player_State` _playerstate))
            (if (>= (`/Game/BluePrints/Player/BP_Player_State.Kills` _asbp_player_state) (`self.LimitKills`))
              (`self.Match Stop` "LimitKills")))
          (:`else`)))
      (:`Is Not Valid`
        (`KismetSystemLibrary.PrintString` "персонаж умер. Но у него нет инстигатора")))))

(fn `UserConstructionScript`
  (`parent.UserConstructionScript`))