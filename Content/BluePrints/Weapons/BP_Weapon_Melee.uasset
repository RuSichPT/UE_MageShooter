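; BP_Weapon_Melee is a melee weapon Blueprint that deals point damage to whatever its swing trace hits.
; UseWeapon runs the parent check, then calls Trace and applies Damage to the hit actor.
; Trace sphere-sweeps a short distance along the owner's forward vector, starting at the player camera pushed forward by spring arm length to offset the third-person boom.
; Each trace also draws a debug line and sphere through DebugFireTraceMulticast.
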(event `DebugFireTraceMulticast`
  (params (Start :type "Vector Structure") (End :type "Vector Structure") (Hit :type "Vector Structure"))
  (`KismetSystemLibrary.DrawDebugLine` Start End (struct :`R` 0.97 :`G` 0.902472 :`A` 1.0) 3.0 2.0)
  (`KismetSystemLibrary.DrawDebugSphere` Hit 20.0 12 (struct :`G` 0.018838 :`B` 0.703125 :`A` 1.0) 3.0 2.0))

(fn `Trace`
  (returns (OutHit :type "HitResult Structure"))
  (bind _asbp_player_character (cast `/Game/BluePrints/Player/BP_PlayerCharacter` (`self.GetInstigator`))
    (:`then`
      (bind _camera (`/Game/BluePrints/Player/BP_PlayerCharacter.Camera` _asbp_player_character))
      (bind _returnvalue (+ (`SceneComponent.K2_GetComponentLocation` _camera) (* (`SceneComponent.GetForwardVector` _camera) (`SpringArmComponent.TargetArmLength` (`/Game/BluePrints/Player/BP_PlayerCharacter.SpringArm` _asbp_player_character)))))
      (bind _outhit (`KismetSystemLibrary.SphereTraceSingleForObjects` _returnvalue (+ _returnvalue (* (`self.GetActorForwardVector` (`self.GetOwner`)) 100.0)) 30.0 (`|MakeArray` "ObjectTypeQuery1" "ObjectTypeQuery2" "ObjectTypeQuery3" "ObjectTypeQuery4" "ObjectTypeQuery5" "ObjectTypeQuery6" :!type "EObjectTypeQuery Enum") false (`|MakeArray` (`self.GetInstigator`) :!type "Actor Object Reference")))
      (bind (_bblockinghit _binitialoverlap _time _distance _location _impactpoint _normal _impactnormal _physmat _hitactor _hitcomponent _hitbonename _hititem _faceindex _tracestart _traceend) (`GameplayStatics.BreakHitResult` _outhit))
      (`self.DebugFireTraceMulticast` _tracestart _traceend _location)
      (return _outhit))
    (:`CastFailed`
      (`KismetSystemLibrary.PrintString` "ERORR not cast player character")
      (return))))

(fn `Use Weapon`
  (returns (Used :type Boolean))
  (bind _used (`parent.Use Weapon`))
  (if _used
    (bind _outhit (`self.Trace`))
    (bind (_bblockinghit _binitialoverlap _time _distance _location _impactpoint _normal _impactnormal _physmat _hitactor _hitcomponent _hitbonename _hititem _faceindex _tracestart _traceend) (`GameplayStatics.BreakHitResult` _outhit))
    (`GameplayStatics.ApplyPointDamage` _hitactor (`self.Damage`) (`KismetMathLibrary.GetDirectionUnitVector` _traceend _tracestart) _outhit (`self.GetInstigatorController`) self)
    (return true)
    (else
      (return false))))

(fn `UserConstructionScript`
  (`parent.UserConstructionScript`))