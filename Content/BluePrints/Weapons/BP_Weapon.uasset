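; Base weapon actor that characters pick up through Interact, which sets instigator and owner and adds it to their weapon manager.
; UseWeapon gates use with a UseRate cooldown timer that repeats automatically until StopUseWeapon clears the Auto flag.
; The WeaponOwner RepNotify toggles collision and attachment, snapping to the owner actor on authority and the mesh's weapon socket on remotes, or detaching when the owner is invalid.
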(fn `AbleToUseWeapon`
  (returns (ReturnValue :type Boolean))
  (return (not (`self.FreezingWeapon`))))

(fn `End Timer`
  (set `self.FreezingWeapon` false)
  (if (`self.Auto`)
    (`self.Use Weapon`)))

(fn `Interact`
  (params (PlayerCharacter :type "/Game/BluePrints/Player/BP_PlayerCharacter Object Reference"))
  (returns (Success :type Boolean))
  (set `self.Instigator` PlayerCharacter)
  (`self.SetOwner` (`Pawn.GetController` PlayerCharacter))
  (`/Game/Components/Player/BP_WeaponManager.Add Weapon` (`/Game/BluePrints/Player/BP_PlayerCharacter.BP_WeaponManager` PlayerCharacter) self)
  (return true))

(fn `OnRep_WeaponOwner`
  (`self.WeaponOwner`
    (:`then`
      (`self.SetActorEnableCollision` false)
      (`/Engine/EditorBlueprintResources/ActorMacros.Switch Has Authority`
        (:`Authority`
          (`self.K2_AttachToActor` (`self.WeaponOwner`) "None" "SnapToTarget" "SnapToTarget" "SnapToTarget"))
        (:`Remote`
          (`self.K2_AttachToComponent` (`Character.Mesh` (`self.WeaponOwner`)) "Skt_Weapon" "SnapToTarget" "SnapToTarget" "SnapToTarget"))))
    (:`else`
      (`self.SetActorEnableCollision` true)
      (`self.K2_DetachFromActor` "KeepRelative")
      (set `self.Instigator` null)
      (`self.SetOwner` null))))

(fn `StopUseWeapon`
  (set `self.Auto` false))

(fn `Use Weapon`
  (returns (Used :type Boolean))
  (set `self.Auto` true)
  (if (`self.AbleToUseWeapon`)
    (set `self.FreezingWeapon` true)
    (`KismetSystemLibrary.K2_SetTimer` null "End Timer" (`self.UseRate`))
    (return true)
    (else
      (set `self.Auto` false)
      (return false))))

(fn `UserConstructionScript`)