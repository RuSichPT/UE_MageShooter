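; Ranged weapon Blueprint that spends ammo on each use, firing either a projectile or a hitscan line trace that applies point damage.
; Shots start from the player camera, offset by spring arm length; the trace extends along the owner's forward vector with multicast debug drawing.
; Setting ReloadingWeapon, automatic on an empty magazine, triggers its OnRep, where authority runs a timer that refills from reserve ammo.
; Use is blocked while empty or reloading.
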(event `DebugFireTraceMulticast`
  (params (Start :type "Vector Structure") (End :type "Vector Structure") (Hit :type "Vector Structure"))
  (`KismetSystemLibrary.DrawDebugLine` Start End (struct :`R` 0.97 :`G` 0.902472 :`A` 1.0) 3.0 2.0)
  (`KismetSystemLibrary.DrawDebugSphere` Hit 20.0 12 (struct :`G` 0.018838 :`B` 0.703125 :`A` 1.0) 3.0 2.0))

(fn `AbleToUseWeapon`
  (returns (ReturnValue :type Boolean))
  (return (and (`parent.AbleToUseWeapon`) (> (`self.CurrentAmmo`) 0) (not (`self.ReloadingWeapon`)))))

(fn `Check Reloading`)

(fn `Fire Projectile`
  (bind _asbp_player_character (cast `/Game/BluePrints/Player/BP_PlayerCharacter` (`self.GetInstigator`)))
  (bind _camera (`/Game/BluePrints/Player/BP_PlayerCharacter.Camera` _asbp_player_character))
  (`|SpawnActorFromClass` (`self.Projectile`) (`KismetMathLibrary.MakeTransform` (+ (.location (`SceneComponent.K2_GetComponentToWorld` _camera)) (* (`SceneComponent.GetForwardVector` _camera) (+ (`SpringArmComponent.TargetArmLength` (`/Game/BluePrints/Player/BP_PlayerCharacter.SpringArm` _asbp_player_character)) 130.0))) (.rotation (`SceneComponent.K2_GetComponentToWorld` _camera)) (.scale (`SceneComponent.K2_GetComponentToWorld` _camera))) "AlwaysSpawn" "OverrideRootScale" self (`self.Damage`) (`self.GetInstigator`)))

(fn `FireTrace`
  (returns (OutHit :type "HitResult Structure"))
  (bind _asbp_player_character (cast `/Game/BluePrints/Player/BP_PlayerCharacter` (`self.GetInstigator`))
    (:`then`
      (bind _camera (`/Game/BluePrints/Player/BP_PlayerCharacter.Camera` _asbp_player_character))
      (bind _returnvalue (+ (`SceneComponent.K2_GetComponentLocation` _camera) (* (`SceneComponent.GetForwardVector` _camera) (`SpringArmComponent.TargetArmLength` (`/Game/BluePrints/Player/BP_PlayerCharacter.SpringArm` _asbp_player_character)))))
      (bind _outhit (`KismetSystemLibrary.LineTraceSingleForObjects` _returnvalue (+ _returnvalue (* (`self.GetActorForwardVector` (`self.GetOwner`)) 5000.0)) (`|MakeArray` "ObjectTypeQuery1" "ObjectTypeQuery2" "ObjectTypeQuery3" "ObjectTypeQuery4" "ObjectTypeQuery5" "ObjectTypeQuery6" :!type "EObjectTypeQuery Enum") false (`|MakeArray` (`self.GetInstigator`) :!type "Actor Object Reference") "ForDuration" true (struct :`R` 1.0 :`A` 1.0) (struct :`G` 1.0 :`A` 1.0) 3.0))
      (bind (_bblockinghit _binitialoverlap _time _distance _location _impactpoint _normal _impactnormal _physmat _hitactor _hitcomponent _hitbonename _hititem _faceindex _tracestart _traceend) (`GameplayStatics.BreakHitResult` _outhit))
      (`self.DebugFireTraceMulticast` _tracestart _traceend _location)
      (return _outhit))
    (:`CastFailed`
      (`KismetSystemLibrary.PrintString` "ERORR not cast player character")
      (return))))

(fn `OnRep_ReloadingWeapon`
  (`/Engine/EditorBlueprintResources/ActorMacros.Switch Has Authority`
    (:`Authority`
      (if (`self.ReloadingWeapon`)
        (bind _output_get (set `self.ReloadAmmo` (`KismetMathLibrary.Min` (`self.TotalAmmo`) (- (`.CurrentAmmo` (defaults `Object` (`GameplayStatics.GetObjectClass` self))) (`self.CurrentAmmo`)))))
        (if (and (> _output_get 0) (not (`KismetSystemLibrary.K2_IsValidTimerHandle` (`self.ReloadTimer`))))
          (`KismetSystemLibrary.PrintString` "Reloading" true true (struct :`R` 1.0 :`B` 0.010051 :`A` 1.0) 0.5)
          (bind _returnvalue (`KismetSystemLibrary.K2_SetTimer` null "Reload Finish" (`self.ReloadTime`)))
          (set `self.ReloadTimer` _returnvalue)
          (else
            (`KismetSystemLibrary.PrintString` (`KismetStringLibrary.Concat_StrStr` "Not able Reloading. CurrentAmmo =  " (`KismetStringLibrary.Conv_IntToString` (`self.CurrentAmmo`))) true true (struct :`R` 1.0 :`B` 0.010051 :`A` 1.0) 0.5)
            (set `self.ReloadingWeapon` false)))))))

(fn `Reload Finish`
  (set `self.ReloadingWeapon` false)
  (`KismetSystemLibrary.K2_ClearAndInvalidateTimerHandle` (`self.ReloadTimer`))
  (set `self.CurrentAmmo` (+ (`self.ReloadAmmo`) (`self.CurrentAmmo`)))
  (set `self.TotalAmmo` (- (`self.TotalAmmo`) (`self.ReloadAmmo`))))

(fn `Use Weapon`
  (returns (Used :type Boolean))
  (bind _used (`parent.Use Weapon`))
  (if _used
    (`/Engine/EditorBlueprintResources/StandardMacros.DecrementInt` (`self.CurrentAmmo`)
      (:`  `
        (`KismetSystemLibrary.PrintString` (`KismetStringLibrary.Concat_StrStr` (`KismetStringLibrary.Conv_IntToString` (`self.CurrentAmmo`)) " | " (`KismetStringLibrary.Conv_IntToString` (`self.TotalAmmo`))) true true (struct :`R` 1.0 :`B` 0.010051 :`A` 1.0) 0.5)
        (if (`KismetSystemLibrary.IsValidClass` (`self.Projectile`))
          (`self.Fire Projectile`)
          (return true)
          (else
            (bind _outhit (`self.FireTrace`))
            (bind (_bblockinghit _binitialoverlap _time _distance _location _impactpoint _normal _impactnormal _physmat _hitactor _hitcomponent _hitbonename _hititem _faceindex _tracestart _traceend) (`GameplayStatics.BreakHitResult` _outhit))
            (`GameplayStatics.ApplyPointDamage` _hitactor (`self.Damage`) (`KismetMathLibrary.GetDirectionUnitVector` _traceend _tracestart) _outhit (`self.GetInstigatorController`) self)
            (return true)))))
    (elif (<= (`self.CurrentAmmo`) 0)
      (set `self.ReloadingWeapon` true) ; Авто Перезярядка
      (return false)
      (else
        (return false)))))

(fn `UserConstructionScript`
  (`parent.UserConstructionScript`))