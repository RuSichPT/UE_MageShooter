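; Base player controller that handles player respawning through the game mode.
; LaunchRespawnTimer sets a timer that calls Respawn, which has BP_BaseGameMode spawn the player for this controller.
; Pressing Enter while controlling a BP_Spectator calls RespawnServer, which respawns at once if the game mode allows fast respawn.
; An event bound to the game mode's match-ended notification clears any pending respawn timer.
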(event `Key|Enter`
  (params (Key :type "Key Structure"))
  (:`Pressed`
    (cast `/Game/BluePrints/Game/Spectators/BP_Spectator` (`self.K2_GetPawn`))
    (`self.RespawnServer`)))

(event `RespawnServer`
  (bind _asbp_base_game_mode (cast `/Game/BluePrints/Game/BP_BaseGameMode` (`GameplayStatics.GetGameMode`)))
  (if (`/Game/BluePrints/Game/BP_BaseGameMode.AllowFastRespawn` _asbp_base_game_mode)
    (`self.Respawn`)))

(event `MatchEndedStopRespawn`
  (params (Reason :type String))
  (remove `/Game/BluePrints/Game/BP_BaseGameMode.MatchEndedServer` (`/Game/BluePrints/Libs/Functions/BP_GlobalGetters.GetBaseGameMode`) (delegate `MatchEndedStopRespawn`))
  (`KismetSystemLibrary.K2_ClearAndInvalidateTimerHandle` (`self.RespawnTimer `)))

(fn `LaunchRespawnTimer`
  (params (Time :type "Float (double-precision)"))
  (bind _returnvalue (`KismetSystemLibrary.K2_SetTimer` null "Respawn" Time))
  (set `self.RespawnTimer ` _returnvalue)
  (add `/Game/BluePrints/Game/BP_BaseGameMode.MatchEndedServer` (`/Game/BluePrints/Libs/Functions/BP_GlobalGetters.GetBaseGameMode`) (`|CreateDelegate` :!event `MatchEndedStopRespawn`)))

(fn `Respawn`
  (bind _asbp_base_game_mode (cast `/Game/BluePrints/Game/BP_BaseGameMode` (`GameplayStatics.GetGameMode`)))
  (`/Game/BluePrints/Game/BP_BaseGameMode.Spawn Player` _asbp_base_game_mode self))

(fn `UserConstructionScript`)