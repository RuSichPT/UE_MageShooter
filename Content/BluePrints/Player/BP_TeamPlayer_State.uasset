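; Team player state Blueprint that stores which Team a player belongs to.
; On BeginPlay the authority randomly assigns one of two team enum values.
; A SetTeamFromClient event overwrites Team with the value passed in.
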(event `SetTeamFromClient`
  (params (Team :type "/Game/Data/E_Team Enum" :default "NewEnumerator0"))
  (set `self.Team` Team))

(event `self.ReceiveBeginPlay`
  (`parent.ReceiveBeginPlay`)
  (`/Engine/EditorBlueprintResources/ActorMacros.Switch Has Authority`
    (:`Authority`
      (set `self.Team` (select `int` (`KismetMathLibrary.RandomInteger` 2) :`0` "NewEnumerator0" :`1` "NewEnumerator1" :!type "/Game/Data/E_Team Enum")))))

(fn `UserConstructionScript`
  (`parent.UserConstructionScript`))