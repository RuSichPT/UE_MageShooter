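; Player controller Blueprint that handles respawning the player through BP_BaseGameMode.
; Pressing Enter while possessing a BP_Spectator calls RespawnServer, which respawns immediately only if the game mode allows fast respawn.
; LaunchRespawnTimer schedules Respawn by function name after a given time and stores the timer handle.
; Respawn delegates the actual spawn to the game mode's SpawnPlayer, passing this controller.
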(event `Key|Enter`
  (params (Key :type "Key Structure"))
  (:`Pressed`
    (cast `/Game/BluePrints/Game/Spectators/BP_Spectator` (`self.K2_GetPawn`))
    (`self.RespawnServer`)))

(event `RespawnServer`
  (bind _asbp_base_game_mode (cast `/Game/BluePrints/Game/BP_BaseGameMode` (`GameplayStatics.GetGameMode`)))
  (if (`/Game/BluePrints/Game/BP_BaseGameMode.AllowFastRespawn` _asbp_base_game_mode)
    (`self.Respawn`)))

(fn `LaunchRespawnTimer`
  (params (Time :type "Float (double-precision)"))
  (bind _returnvalue (`KismetSystemLibrary.K2_SetTimer` null "Respawn" Time))
  (set `self.RespawnTimer ` _returnvalue))

(fn `Respawn`
  (bind _asbp_base_game_mode (cast `/Game/BluePrints/Game/BP_BaseGameMode` (`GameplayStatics.GetGameMode`)))
  (`/Game/BluePrints/Game/BP_BaseGameMode.Spawn Player` _asbp_base_game_mode self))

(fn `UserConstructionScript`)