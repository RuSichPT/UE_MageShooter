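; Player character Blueprint for the Maria character, adding jump-button state handling on top of its parent class.
; MyJump and MyStopJumping set JumpButtonDown locally, then call JumpServer and StopJumpServer, which set the same flag, apparently as server-side mirrors.
; The construction script defers to the parent, ToColorCharacter is an empty stub, and BeginPlay, overlap and Tick events are unused.
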(event `JumpServer`
  (set `self.JumpButtonDown` true))

(event `StopJumpServer`
  (set `self.JumpButtonDown` false))

(fn `MyJump`
  (set `self.JumpButtonDown` true)
  (`self.JumpServer`))

(fn `MyStopJumping`
  (set `self.JumpButtonDown` false)
  (`self.StopJumpServer`))

(fn `To Color Character`)

(fn `UserConstructionScript`
  (`parent.UserConstructionScript`))