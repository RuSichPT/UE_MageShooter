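; BP_WeaponSpawner is a pickup point that displays a weapon and gives it to an overlapping player.
; The construction script creates the first weapon as a child actor, which BeginPlay offsets on authority and strips of collision.
; On authority, sphere overlap passes it to the player's BPWeaponManager unless that weapon class is already held.
; A timer then calls RespawnWeapon to spawn a standalone, collisionless replacement at the offset.
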(event `self.ReceiveBeginPlay`
  (`/Engine/EditorBlueprintResources/ActorMacros.Switch Has Authority`
    (:`Authority`
      (`self.K2_AddActorLocalOffset` (`self.Weapon`) (`self.ChildLocalOffset`) false false))
    (:`Remote`
      _))
  (`self.SetActorEnableCollision` (`self.Weapon`) false))

(event `self.Sphere.OnComponentBeginOverlap`
  (params (OverlappedComponent :type "PrimitiveComponent Object Reference") (OtherActor :type "Actor Object Reference") (OtherComp :type "PrimitiveComponent Object Reference") (OtherBodyIndex :type Integer) (bFromSweep :type Boolean) (SweepResult :type "HitResult Structure (by ref)"))
  (`/Engine/EditorBlueprintResources/ActorMacros.Switch Has Authority`
    (:`Authority`
      (bind _asbp_player_character (cast `/Game/BluePrints/Player/BP_PlayerCharacter` OtherActor))
      (bind _weapon (`self.Weapon`)
        (:`then`
          (bind _bp_weaponmanager (`/Game/BluePrints/Player/BP_PlayerCharacter.BP_WeaponManager` _asbp_player_character))
          (if (not (`/Game/Components/Player/BP_WeaponManager.IsEqualWeaponClass` _bp_weaponmanager _weapon))
            (`/Game/Components/Player/BP_WeaponManager.AddWeapon` _bp_weaponmanager _weapon)
            (set `self.Weapon` null)
            (`KismetSystemLibrary.K2_SetTimer` null "RespawnWeapon" (`self.RespawnTime`))))
        (:`else`)))))

(fn `RespawnWeapon`
  (bind _returnvalue (`|SpawnActorFromClass` (`self.WeaponClass`) (`KismetMathLibrary.MakeTransform` (+ (`self.K2_GetActorLocation`) (`self.ChildLocalOffset`))) "Undefined" "OverrideRootScale" null null null))
  (bind _output_get (set `self.Weapon` _returnvalue))
  (`self.SetActorEnableCollision` _output_get false)
  (`KismetSystemLibrary.PrintString` (`KismetStringLibrary.Conv_BoolToString` (`self.GetActorEnableCollision` self))))

(fn `UserConstructionScript`
  (bind _returnvalue (`AddComponent|NODE_AddChildActorComponent-0`))
  (`ChildActorComponent.SetChildActorClass` _returnvalue (`self.WeaponClass`))
  (set `self.Weapon` (cast `/Game/BluePrints/Weapons/BP_Weapon` (`ChildActorComponent.ChildActor` _returnvalue) :!pure true)))