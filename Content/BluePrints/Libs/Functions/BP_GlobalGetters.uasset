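; BP_GlobalGetters is a Blueprint function library of typed shortcuts to the game's core gameplay framework objects.
; Each function fetches a game mode, game state, player state, player controller or HUD and returns it cast to the project's Blueprint class.
; Variants cover the base and team classes, plus a deathmatch game mode.
; Game mode and state getters take no arguments, while the others resolve from a supplied controller, pawn or player.
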(fn `GetBaseGameMode`
  (returns (`AsBP Base Game Mode` :type "/Game/BluePrints/Game/BP_BaseGameMode Object Reference"))
  (return (cast `/Game/BluePrints/Game/BP_BaseGameMode` (`GameplayStatics.GetGameMode` null) :!pure true)))

(fn `GetBaseGameState`
  (returns (`AsBP Base Game State` :type "/Game/BluePrints/Game/BP_BaseGameState Object Reference"))
  (return (cast `/Game/BluePrints/Game/BP_BaseGameState` (`GameplayStatics.GetGameState` null) :!pure true)))

(fn `GetBaseHUD`
  (params (Player :type "PlayerController Object Reference"))
  (returns (`Base HUD` :type "/Game/BluePrints/Game/BP_BaseHUD Object Reference"))
  (return (cast `/Game/BluePrints/Game/BP_BaseHUD` (`PlayerController.GetHUD` Player) :!pure true)))

(fn `GetBasePlayerController`
  (params (Pawn :type "Pawn Object Reference"))
  (returns (`AsBP Base Player Controller` :type "/Game/BluePrints/Player/BP_BasePlayerController Object Reference"))
  (return (cast `/Game/BluePrints/Player/BP_BasePlayerController` (`Pawn.GetController` Pawn) :!pure true)))

(fn `GetDeathMatchGameMode`
  (returns (`AsBP Death Match Game Mode` :type "/Game/BluePrints/Game/BP_DeathMatchGameMode Object Reference"))
  (return (cast `/Game/BluePrints/Game/BP_DeathMatchGameMode` (`GameplayStatics.GetGameMode` null) :!pure true)))

(fn `GetPlayerStateByController`
  (params (Controller :type "Controller Object Reference"))
  (returns (`AsBP Player State` :type "/Game/BluePrints/Player/BP_Player_State Object Reference"))
  (return (cast `/Game/BluePrints/Player/BP_Player_State` (`Controller.PlayerState` Controller) :!pure true)))

(fn `GetTeamGameMode`
  (returns (`AsBP Team Game Mode` :type "/Game/BluePrints/Game/BP_TeamGameMode Object Reference"))
  (return (cast `/Game/BluePrints/Game/BP_TeamGameMode` (`GameplayStatics.GetGameMode` null) :!pure true)))

(fn `GetTeamGameState`
  (returns (`AsBP Team Game State` :type "/Game/BluePrints/Game/BP_TeamGameState Object Reference"))
  (return (cast `/Game/BluePrints/Game/BP_TeamGameState` (`GameplayStatics.GetGameState` null) :!pure true)))

(fn `GetTeamHUD`
  (params (Player :type "PlayerController Object Reference"))
  (returns (`Team HUD` :type "/Game/BluePrints/Game/BP_TeamHUD Object Reference"))
  (return (cast `/Game/BluePrints/Game/BP_TeamHUD` (`PlayerController.GetHUD` Player) :!pure true)))

(fn `GetTeamPlayerStateByController`
  (params (Controller :type "Controller Object Reference"))
  (returns (`AsBP Team Player State` :type "/Game/BluePrints/Player/BP_TeamPlayer_State Object Reference"))
  (return (cast `/Game/BluePrints/Player/BP_TeamPlayer_State` (`Controller.PlayerState` Controller) :!pure true)))